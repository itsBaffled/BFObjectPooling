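; BP_MovingActor is a prop in the PoolShowcase folder that shuttles back and forth along its local X axis.
; Each Tick it adds a frame-rate-independent local offset without sweep, with a boolean choosing the positive or negative direction at a fixed speed.
; An accumulated timer flips that boolean and resets roughly every two seconds, reversing the motion.
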(event `self.ReceiveTick`
  (params (DeltaSeconds :type "Float (single-precision)"))
  (set `self.Seconds` (+ DeltaSeconds (`self.Seconds`)))
  (`self.K2_AddActorLocalOffset` (* DeltaSeconds (`KismetMathLibrary.SelectVector` (500.0 0.0 0.0) (-500.0 0.0 0.0) (`self.bFlip`))))
  (if (> (`self.Seconds`) 2.0)
    (set `self.bFlip` (not (`self.bFlip`)))
    (set `self.Seconds` 0.0)))

(fn `UserConstructionScript`)